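; BP_Checkpoint is an overlap-triggered checkpoint that sets itself as the Hugo player's current checkpoint.
; On overlap it fires a dispatcher that every checkpoint binds on all instances at BeginPlay, so only the latest one stays active.
; Tick disables and hides the active checkpoint's collision component and restores query collision and visibility on the others.
; The construction script places SpawnPosition at the bottom of the collision bounds.
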(event `CheckpointReached`
  (set `/Game/Blueprints/Player/Hugo.currentCheckpoint` self (`/Game/Blueprints/Libraries/TS2Macros.GetPlayerAsHugo`))
  (`KismetSystemLibrary.PrintString` "Checkpoint Reached!"))

(event `self.ReceiveActorBeginOverlap`
  (params (OtherActor :type "Actor Object Reference"))
  (`self.CheckpointReached`)
  (`self.CheckpointReached_Dispatcher` self))

(event `self.ReceiveTick`
  (params (DeltaSeconds :type "Float (single-precision)"))
  (`PrimitiveComponent.SetCollisionEnabled` (`self.CollisionComponent`) (select `bool` (`self.checkpointActive`) :`false` "QueryOnly" :`true` "NoCollision" :!type "ECollisionEnabled Enum"))
  (`SceneComponent.SetHiddenInGame` (`self.CollisionComponent`) (`self.checkpointActive`) false))

(event `self.ReceiveBeginPlay`
  (bind _outactors (`GameplayStatics.GetAllActorsOfClass` "BP_Checkpoint_C"))
  (add `self.CheckpointReached_Dispatcher` _outactors (delegate `CheckpointReached_Dispatcher_Event`)))

(event `CheckpointReached_Dispatcher_Event` :!signature `self.CheckpointReached_Dispatcher`
  (params (newActiveCheckpoint :type "/Game/Blueprints/Gameplay/BP_Checkpoint Object Reference"))
  (bind _output_get (set `self.checkpointActive` (== newActiveCheckpoint self)))
  (`KismetSystemLibrary.PrintString` (`KismetStringLibrary.BuildString_Bool` (`KismetSystemLibrary.GetDisplayName` self) ": " _output_get)))

(fn `UserConstructionScript`
  (set `self.spawnPosition` (- (`self.K2_GetActorLocation`) (`KismetMathLibrary.MakeVector` 0.0 0.0 (.z (`.BoxExtent` (`KismetSystemLibrary.GetComponentBounds` (`self.CollisionComponent`))))))))