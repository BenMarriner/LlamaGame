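; BP_BaseItem is a base pickup actor that spins its mesh and disappears when the player touches it.
; The CoinRotation timeline starts on BeginPlay and lerps the mesh through a full turn around the axis chosen by SpinAxis.
; The other axes reuse the mesh's world rotation, except roll, which is zeroed for Z spin.
; Overlap with player character 0 destroys the actor, with no other pickup effect.
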(event `self.ReceiveBeginPlay`
  (bind _mesh (`self.Mesh`))
  (bind (_returnvalue_roll _returnvalue_pitch _returnvalue_yaw) (`KismetMathLibrary.BreakRotator` (`SceneComponent.K2_GetComponentRotation` _mesh)))
  ;[0 1 0.5781] Spin Animation
  (bind (_direction _rotation) (`Timeline|CoinRotation`)
    (:`Update`
      (switch `/Game/Blueprints/Enums/Axes` (`self.spinAxis`)
        (:`NewEnumerator0`
          (bind _returnvalue (`KismetMathLibrary.Lerp` -180.0 180.0 _rotation))
          (`SceneComponent.K2_SetRelativeRotation` _mesh (`KismetMathLibrary.MakeRotator` _returnvalue _returnvalue_pitch _returnvalue_yaw) false false))
        (:`NewEnumerator1`
          (`SceneComponent.K2_SetRelativeRotation` _mesh (`KismetMathLibrary.MakeRotator` _returnvalue_roll _returnvalue _returnvalue_yaw) false false))
        (:`NewEnumerator2`
          (`SceneComponent.K2_SetRelativeRotation` _mesh (`KismetMathLibrary.MakeRotator` 0.0 _returnvalue_pitch _returnvalue) false false))))))

(event `self.ReceiveActorBeginOverlap`
  (params (OtherActor :type "Actor Object Reference"))
  (if (== OtherActor (`GameplayStatics.GetPlayerCharacter` 0))
    (`self.K2_DestroyActor`)))

(fn `UserConstructionScript`)