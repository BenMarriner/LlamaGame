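; Spawner actor that repeatedly spawns obstacles at its own transform, passing them a scaled velocity and a lifespan, while capping the live count.
; Tick uses a DoOnce to start a looping spawn timer when enabled and below the limit, otherwise clearing it and resetting the gate.
; Spawns increment the count and bind to each obstacle's destruction to decrement it, letting spawning resume.
; Tick also prints the count for debugging.
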(event `self.ReceiveTick`
  (params (DeltaSeconds :type "Float (single-precision)"))
  (`|ExecutionSequence`
    (:`then_0`
      (bind _output_get (set `self.obstacleLimitReached` (>= (`self.count`) (`self.maxObstacles`))))
      (if (and (not _output_get) (`self.enabled`))
        (`/Engine/EditorBlueprintResources/StandardMacros.DoOnce` false :!label _label
          (:`Completed`
            (bind _returnvalue (`KismetSystemLibrary.K2_SetTimer` null "SpawnObstacle" (`self.spawnRate`) true))
            (set `self.spawnTimerHandle` _returnvalue)))
        (else
          (`self.SpawnLimitReached`))))
    (:`then_1`
      (`KismetSystemLibrary.PrintString` (`KismetStringLibrary.BuildString_Int` "Obstacles spawned: " "" (`self.count`)) true true (struct :`G` 0.66 :`B` 1.0 :`A` 1.0) 0.0))))

(event `ObstacleDestroyed`
  (params (DestroyedActor :type "Actor Object Reference"))
  (`/Engine/EditorBlueprintResources/StandardMacros.DecrementInt` (`self.count`)))

(event `SpawnLimitReached`
  (`KismetSystemLibrary.K2_ClearTimer` null "SpawnObstacle")
  (goto _label :!via `Reset`))

(fn `SpawnObstacle`
  (bind _returnvalue (`|SpawnActorFromClass` (`self.obstacleTemplate`) (`self.GetTransform`) "Undefined" "OverrideRootScale" null (* (`self.velocity`) (`self.velocityMultiplier`)) (`self.lifespan`) null))
  (add `self.OnDestroyed` _returnvalue (`|CreateDelegate` :!event `ObstacleDestroyed`))
  (`/Engine/EditorBlueprintResources/StandardMacros.IncrementInt` (`self.count`)))

(fn `UserConstructionScript`)