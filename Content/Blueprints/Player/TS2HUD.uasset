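; TS2HUD is a player HUD Blueprint that manages the main on-screen display and an exit menu.
; On BeginPlay it creates the TS2Display widget and adds it to the viewport.
; CreateExitMenu hides that display, adds a new ExitMenu widget and shows the mouse cursor.
; CloseExitMenu hides the cursor and removes the menu, but does not make the hidden display visible again.
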(event `self.ReceiveBeginPlay`
  (bind _returnvalue (`|CreateWidget` "/Game/Blueprints/Player/TS2Display.TS2Display_C"))
  (bind _output_get (set `self.HUD` _returnvalue))
  (`UserWidget.AddToViewport` _output_get 0))

(event `CreateExitMenu`
  (`Widget.SetVisibility` (stale `self.ReceiveBeginPlay` _output_get) "Hidden")
  (bind _returnvalue (`|CreateWidget` "/Game/Blueprints/Player/ExitMenu.ExitMenu_C"))
  (bind _output_get (set `self.exitMenu` _returnvalue))
  (`UserWidget.AddToViewport` _output_get 0)
  (set `PlayerController.bShowMouseCursor` true (`GameplayStatics.GetPlayerController` 0)))

(event `CloseExitMenu`
  (set `PlayerController.bShowMouseCursor` false (`GameplayStatics.GetPlayerController` 0))
  (`Widget.RemoveFromParent` (stale `CreateExitMenu` _output_get)))

(fn `UserConstructionScript`)