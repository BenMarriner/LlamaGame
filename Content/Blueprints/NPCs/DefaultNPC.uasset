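; DefaultNPC is an NPC Blueprint with a capsule component, but none of its logic runs: its only node chain has no event and the construction script is empty.
; The disconnected chain offsets player 0 along negative Y from the NPC, then line-traces down from the player's capsule base against WorldStatic with debug drawing.
; It then moves the NPC's own capsule to the player's XY at the traced ground height.
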(fn `UserConstructionScript`)