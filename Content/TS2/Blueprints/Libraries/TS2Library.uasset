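; TS2Library is a shared gameplay library for TS2 covering level flow, camera blending and enemy knockback.
; Level start resets items and level number on TS2Instance and fades the camera, while transitions open maps by enum, with next-level names unfilled and LevelEndProcedures empty.
; InterpolateBetweenCameras steps location and rotation toward a target, prints debug values and returns whether it has arrived.
; EnemyPushPlayer launches the player opposite the enemy's forward vector.
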(fn `EnemyPushPlayer`
  (params (Enemy :type "/Game/TS2/Blueprints/NPCs/DefaultNPC Object Reference"))
  (bind (_returnvalue_x _returnvalue_y _returnvalue_z) (`KismetMathLibrary.BreakVector` (`Actor.GetActorForwardVector` Enemy)))
  (`Character.LaunchCharacter` (`GameplayStatics.GetPlayerCharacter` null) (* (`KismetMathLibrary.MakeVector` _returnvalue_x _returnvalue_y _returnvalue_z) -100.0) false false))

(fn `InterpolateBetweenCameras`
  (params (currentCamera :type "CameraComponent Object Reference") (targetCamera :type "CameraComponent Object Reference") (deltaTime :type "Float (double-precision)") (VinterpSpeed :type "Float (double-precision)") (rinterpSpeed :type "Float (double-precision)"))
  (returns (complete :type Boolean))
  (locals (cameraMoving :type Boolean))
  (bind _currentcamera (`local.currentCamera`))
  (bind _targetcamera (`local.targetCamera`))
  (bind _returnvalue (`SceneComponent.K2_GetComponentLocation` _targetcamera))
  (bind _returnvalue_2 (`SceneComponent.K2_GetComponentLocation` _currentcamera))
  (bind _returnvalue_3 (`SceneComponent.K2_GetComponentRotation` _currentcamera))
  (bind _returnvalue_4 (`SceneComponent.K2_GetComponentRotation` _targetcamera))
  (set `local.cameraMoving` true)
  (`SceneComponent.K2_SetWorldLocationAndRotation` currentCamera (`KismetMathLibrary.VInterpTo` (`SceneComponent.K2_GetComponentLocation` currentCamera) (`SceneComponent.K2_GetComponentLocation` targetCamera) deltaTime VinterpSpeed) (`KismetMathLibrary.RInterpTo` (`SceneComponent.K2_GetComponentRotation` currentCamera) (`SceneComponent.K2_GetComponentRotation` targetCamera) deltaTime rinterpSpeed) false false)
  ;[0 0.03906 1 0.5] Debug Camera Values
  (`KismetSystemLibrary.PrintString` null (`KismetStringLibrary.Concat_StrStr` "Current Camera Location: " (`KismetStringLibrary.Conv_VectorToString` _returnvalue_2)) true true (struct :`G` 0.66 :`B` 1.0 :`A` 1.0) 50.0)
  (`KismetSystemLibrary.PrintString` null (`KismetStringLibrary.Concat_StrStr` "Target Camera Location: " (`KismetStringLibrary.Conv_VectorToString` _returnvalue)) true true (struct :`G` 0.66 :`B` 1.0 :`A` 1.0) 50.0)
  (`KismetSystemLibrary.PrintString` null (`KismetStringLibrary.Concat_StrStr` "Current Camera Rotation: " (`KismetStringLibrary.Conv_RotatorToString` _returnvalue_3)) true true (struct :`G` 0.66 :`B` 1.0 :`A` 1.0) 50.0)
  (`KismetSystemLibrary.PrintString` null (`KismetStringLibrary.Concat_StrStr` "Target Camera Rotation: " (`KismetStringLibrary.Conv_RotatorToString` _returnvalue_4)) true true (struct :`G` 0.66 :`B` 1.0 :`A` 1.0) 50.0)
  (return (and (== _returnvalue_2 _returnvalue :`ErrorTolerance` 1.0) (== _returnvalue_3 _returnvalue_4 :`ErrorTolerance` 1.0))))

(fn `LevelEndProcedures`)

(fn `LevelStartProcedures`
  (bind _asts2instance (cast `/Game/TS2/Blueprints/Player/TS2Instance` (`GameplayStatics.GetGameInstance` null) :!pure true))
  (`|ExecutionSequence`
    (:`then_0`
      (`/Game/TS2/Blueprints/Player/TS2Instance.InitializeItems` _asts2instance)
      (set `/Game/TS2/Blueprints/Player/TS2Instance.currentLevelNumber` 0 _asts2instance))
    (:`then_1`
      (`PlayerCameraManager.StartCameraFade` :`self` (`GameplayStatics.GetPlayerCameraManager` null) :`FromAlpha` 2.5 :`Duration` 1.0))))

(fn `LevelTransitionProcedures`
  (params (mapTransition :type "/Game/TS2/Blueprints/Enums/TransitionSelections Enum" :default "NewEnumerator0") (nextLevel :type Byte))
  (switch `/Game/TS2/Blueprints/Enums/TransitionSelections` mapTransition
    (:`NewEnumerator0`
      ;[1 0.8672 0] Transition from Level to Level Complete
      (`GameplayStatics.OpenLevel` null "LevelComplete"))
    (:`NewEnumerator1`
      ;[0 1 0.7422] Transition from Level Complete to Level Select
      (`GameplayStatics.OpenLevel` null "LevelSelect"))
    (:`NewEnumerator2`
      ;[0.7812 1 0] Transition from Level Select to Next Level
      (`GameplayStatics.OpenLevel` null (select `byte` nextLevel :`0` "None" :`1` "None" :!type "Name")))
    (:`NewEnumerator3`
      ;[1 0 0.375] Transition from Level to Game Over
      (`GameplayStatics.OpenLevel` null "GameOver"))))