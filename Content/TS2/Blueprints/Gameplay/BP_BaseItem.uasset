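; BP_BaseItem is a base pickup item that animates in place and destroys itself when the player character overlaps it.
; On BeginPlay, SetMovementBehaviour selects spin, bounce or both, driven by the CoinRotation and Bounce timelines.
; Spin lerps the mesh rotation around the chosen SpinAxis.
; Bounce lerps the actor's world Z between zero and MaxBounceHeight, ignoring its placed height.
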(event `self.ReceiveBeginPlay`
  (bind (_returnvalue_x _returnvalue_y) (`KismetMathLibrary.BreakVector` (`self.K2_GetActorLocation`)))
  (bind _mesh (`self.Mesh`))
  (bind (_returnvalue_roll _returnvalue_pitch _returnvalue_yaw) (`KismetMathLibrary.BreakRotator` (`SceneComponent.K2_GetComponentRotation` _mesh)))
  (switch `/Game/TS2/Blueprints/Enums/ItemMovementBehaviours` (`self.setMovementBehaviour`)
    (:`NewEnumerator0`
      ;[0 1 0.5781] Spin Animation
      (bind (_direction _rotation) (`Timeline|CoinRotation` :!label _label)
        (:`Update`
          (switch `/Game/TS2/Blueprints/Enums/Axes` (`self.spinAxis`)
            (:`NewEnumerator0`
              (bind _returnvalue (`KismetMathLibrary.Lerp` -180.0 180.0 _rotation))
              (`SceneComponent.K2_SetRelativeRotation` _mesh (`KismetMathLibrary.MakeRotator` _returnvalue _returnvalue_pitch _returnvalue_yaw) false false))
            (:`NewEnumerator1`
              (`SceneComponent.K2_SetRelativeRotation` _mesh (`KismetMathLibrary.MakeRotator` _returnvalue_roll _returnvalue _returnvalue_yaw) false false))
            (:`NewEnumerator2`
              (`SceneComponent.K2_SetRelativeRotation` _mesh (`KismetMathLibrary.MakeRotator` 0.0 _returnvalue_pitch _returnvalue) false false))))))
    (:`NewEnumerator1`
      ;[0.2422 0 1] Bounce Animation
      (bind (_direction_2 _bouncecurve) (`Timeline|Bounce` :!label _label_2)
        (:`Update`
          (`self.K2_SetActorLocation` (`KismetMathLibrary.MakeVector` _returnvalue_x _returnvalue_y (`KismetMathLibrary.Lerp` 0.0 (`self.maxBounceHeight`) _bouncecurve))))))
    (:`NewEnumerator2`
      (`|ExecutionSequence`
        (:`then_0`
          (goto _label))
        (:`then_1`
          (goto _label_2))))))

(event `self.ReceiveActorBeginOverlap`
  (params (OtherActor :type "Actor Object Reference"))
  (if (== OtherActor (`GameplayStatics.GetPlayerCharacter` 0))
    (`self.K2_DestroyActor`)))

(fn `UserConstructionScript`)