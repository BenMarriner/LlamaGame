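; Default NPC that lets the player start a dialogue by bumping into it.
; On a hit from the player character, it checks AllowDialogueEntry and passes itself to the ThirdPersonCharacter's BeginDialogueInteraction.
; UnlockToken tells the player HUD to end the dialogue.
; An unconnected chain, which never runs, repositions the player and NPC capsules using a downward ground trace.
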(event `self.ReceiveHit`
  (params (MyComp :type "PrimitiveComponent Object Reference") (Other :type "Actor Object Reference") (OtherComp :type "PrimitiveComponent Object Reference") (bSelfMoved :type Boolean) (HitLocation :type "Vector Structure") (HitNormal :type "Vector Structure") (NormalImpulse :type "Vector Structure") (Hit :type "HitResult Structure (by ref)"))
  (bind _returnvalue (`GameplayStatics.GetPlayerCharacter` 0))
  (if (and (`self.allowDialogueEntry`) (== Other _returnvalue))
    (`/Game/ThirdPersonTemplate/ThirdPersonBP/Blueprints/ThirdPersonCharacter.BeginDialogueInteraction` (cast `/Game/ThirdPersonTemplate/ThirdPersonBP/Blueprints/ThirdPersonCharacter` _returnvalue :!pure true) self)))

(event `UnlockToken`
  (`/Game/TS2/Blueprints/Player/TS2Display.UninitiateDialogue` (`/Game/TS2/Blueprints/Libraries/TS2Macros.GetPlayerHUD`)))

(fn `UserConstructionScript`)